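; Game mode that creates the main widget and switches the BP_FPSCharacter between bird's-eye and first-person views.
; FpsMode saves the current transform, glides the character via timeline-driven transform lerps to the DT_DH_Loc row named by NDHName, then enables FPS view.
; BirdViewMode enables bird view immediately and lerps the character back to the BirdViewTransform saved when FpsMode last left bird view.
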(event `self.ReceiveBeginPlay`
  (bind _returnvalue (`|CreateWidget` "/Game/Dev/RTY/WBP/WBP_MainWidget.WBP_MainWidget_C" (`GameplayStatics.GetPlayerController` 0)))
  (`UserWidget.AddToViewport` _returnvalue 0)
  (bind _returnvalue_2 (`GameplayStatics.GetActorOfClass` "/Game/Dev/RTY/BluePrints/BP_FPSCharacter.BP_FPSCharacter_C"))
  (set `self.FPS_Character` _returnvalue_2))

(event `BirdViewMode`
  (`/Game/Dev/RTY/BluePrints/BP_FPSCharacter.SetBirdView` (`self.FPS_Character`))
  (bind (_direction _newtrack_0) (`Timeline|Timeline_0` :!via `PlayFromStart`)
    (:`Update`
      (`self.K2_SetActorTransform` (`self.FPS_Character`) (`KismetMathLibrary.TLerp` (`self.GetTransform` (`self.FPS_Character`)) (`self.BirdViewTransform`) _newtrack_0) false false))))

(event `FpsMode`
  (bind _fps_character (`self.FPS_Character`))
  (bind _ndhname (`self.nDHName`))
  (bind _fps_character_2 (`self.FPS_Character`))
  (if (`AFPSCharacter.bIsBirdView` (`self.FPS_Character`))
    (bind _output_get (set `self.BirdViewTransform` (`self.GetTransform` (`self.FPS_Character`))))
    (bind _returnvalue (`|GetDataTableRow` "/Game/Dev/RTY/Structure/DT_DH_Loc.DT_DH_Loc" _ndhname)
      (:`then`
        (bind (_direction _newtrack_0) (`Timeline|Timeline_Lerp` :!via `PlayFromStart`)
          (:`Update`
            (`self.K2_SetActorTransform` _fps_character (`KismetMathLibrary.TLerp` _output_get (`.MemberVar_13_14_22356E114F5FEE47325CDB80F51FCA67` (break `/Game/Dev/RTY/Structure/S_APTLoc` _returnvalue)) _newtrack_0) false false))
          (:`Finished`
            (`/Game/Dev/RTY/BluePrints/BP_FPSCharacter.SetFPSView` _fps_character)))))
    (else
      (bind _output_get_2 (set `self.Loc_InAPT` (`self.GetTransform` (`self.FPS_Character`))))
      (bind _returnvalue_2 (`|GetDataTableRow` "/Game/Dev/RTY/Structure/DT_DH_Loc.DT_DH_Loc" _ndhname)
        (:`then`
          (bind (_direction_2 _newtrack_0_2) (`Timeline|Timeline` :!via `PlayFromStart`)
            (:`Update`
              (`self.K2_SetActorTransform` _fps_character_2 (`KismetMathLibrary.TLerp` _output_get_2 (`.MemberVar_13_14_22356E114F5FEE47325CDB80F51FCA67` (break `/Game/Dev/RTY/Structure/S_APTLoc` _returnvalue_2)) _newtrack_0_2) false false))
            (:`Finished`
              (`/Game/Dev/RTY/BluePrints/BP_FPSCharacter.SetFPSView` _fps_character_2))))))))

(event `self.ReceiveTick`
  (params (DeltaSeconds :type "Float (single-precision)")))

(fn `UserConstructionScript`)